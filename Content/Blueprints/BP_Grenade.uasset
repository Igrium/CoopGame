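; Grenade actor that detonates two seconds after spawning, or earlier when it hits a Character.
; BeginPlay runs the fuse delay and the Hit event checks the other actor's class, both calling a shared Explode function.
; Explode applies radial damage with falloff at the grenade's location, spawns an explosion particle effect and destroys the actor.
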(event `self.ReceiveBeginPlay`
  (`KismetSystemLibrary.Delay` 2.0)
  (`self.Explode`))

(event `self.ReceiveHit`
  (params (MyComp :type "PrimitiveComponent Object Reference") (Other :type "Actor Object Reference") (OtherComp :type "PrimitiveComponent Object Reference") (bSelfMoved :type Boolean) (HitLocation :type "Vector Structure") (HitNormal :type "Vector Structure") (NormalImpulse :type "Vector Structure") (Hit :type "HitResult Structure (by ref)"))
  (if (`KismetMathLibrary.ClassIsChildOf` (`GameplayStatics.GetObjectClass` Other) "/Script/Engine.Character")
    (`self.Explode`)))

(fn `Explode`
  (`GameplayStatics.ApplyRadialDamageWithFalloff` 30.0 0.0 (`self.K2_GetActorLocation`) 100.0 0.0 300.0)
  (`GameplayStatics.SpawnEmitterAtLocation` "/Game/WeaponEffects/Explosion/P_Explosion.P_Explosion" (`self.K2_GetActorLocation`))
  (`self.K2_DestroyActor`))

(fn `UserConstructionScript`)